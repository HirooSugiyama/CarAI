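; GM_AISample is an AI sample Blueprint, likely a game mode by its prefix, that keeps spawning cars on splines.
; On BeginPlay it starts a looping timer that periodically picks a random entry from MBaseSplines, if the array has a first element, and passes it to ACOMCarManager's CreateCar.
; Tick only stores the frame's delta time in TICK.
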(event EventBeginPlay
  (CallFunction|CreateCars))

(event EventTick
  (params (DeltaSeconds :type Float%20%28single-precision%29))
  (Variables|Default|SetTICK DeltaSeconds))

(event Custom|CreateCars
  (Utilities|Time|SetTimerbyEvent (delegate Custom|createCar) 2.0 true))

(event Custom|createCar
  (bind _mbasesplines (Variables|Default|GetmBaseSplines))
  (if (Utilities|Array|IsValidIndex _mbasesplines)
    (Default|CreateCar (Variables|Default|GetACOM_CarManager) (Utilities|Array|Get(acopy) _mbasesplines (Math|Random|RandomInteger (Utilities|Array|Length _mbasesplines))))))

(fn ConstructionScript)