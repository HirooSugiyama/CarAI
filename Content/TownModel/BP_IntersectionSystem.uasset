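; Intersection controller that cycles four directional traffic lights through blue (go), yellow and red in alternating pairs.
; At BeginPlay it sets Center and Back blue, Right and Left red, and records the blue pair in MNowBlueLight.
; Timer events, delayed by COLORTIMER durations, turn blue to yellow, then yellow to red.
; The Red timer swaps MNowBlueLight to the lights outside it, turns them blue and restarts the cycle.
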(event Custom|ColorUpdate
  (Utilities|Time|SetTimerbyEvent (delegate Custom|BlueToYerrow) 0.01 false (.Value (Utilities|Map|Find (Variables|Default|GetCOLOR_TIMER) "NewEnumerator0")))
  (Utilities|Time|SetTimerbyEvent (delegate Custom|RedUpdate) 0.01 false (.Value (Utilities|Map|Find (Variables|Default|GetCOLOR_TIMER) "NewEnumerator7"))))

(event Custom|BlueToYerrow
  (Private|ChangeLightColor "NewEnumerator0") ; 青い信号機を黄色へ
  (Utilities|Time|SetTimerbyEvent (delegate Custom|YerrowUpdate) 0.001 false (.Value (Utilities|Map|Find (Variables|Default|GetCOLOR_TIMER) "NewEnumerator3"))))

(event Custom|RedUpdate
  (Private|ChangeLightColor "NewEnumerator7") ; 赤い信号機を青色へ
  (CallFunction|ColorUpdate))

(event Custom|YerrowUpdate
  (Private|ChangeLightColor "NewEnumerator3") ; 黄色い信号機を赤色へ
)

(event EventBeginPlay
  (Private|InitTraficLight)
  (CallFunction|ColorUpdate))

(fn ConstructionScript)

(fn InitTraficLight
  (bind _enumvalue (|ForEachEN_IntersectionDirection)
    (:LoopBody
      (Utilities|IsValid (.Value (Utilities|Map|Find (Variables|Default|GetmTraficLights) _enumvalue))
        (:Is%20Valid
          (switch Utilities|FlowControl|Switch|SwitchonEN_IntersectionDirection _enumvalue
            (:NewEnumerator0
              (Default|ChangeLightColor (.Value (Utilities|Map|Find (Variables|Default|GetmTraficLights) _enumvalue)) "NewEnumerator0")
              (Private|AddBlueLight (.Value (Utilities|Map|Find (Variables|Default|GetmTraficLights) _enumvalue)) :!label _label))
            (:NewEnumerator1
              (Default|ChangeLightColor (.Value (Utilities|Map|Find (Variables|Default|GetmTraficLights) _enumvalue)) "NewEnumerator0")
              (goto _label))
            (:NewEnumerator2
              (Default|ChangeLightColor (.Value (Utilities|Map|Find (Variables|Default|GetmTraficLights) _enumvalue)) "NewEnumerator7"))
            (:NewEnumerator3
              (Default|ChangeLightColor (.Value (Utilities|Map|Find (Variables|Default|GetmTraficLights) _enumvalue)) "NewEnumerator7"))))))))

(fn ChangeLightColor
  (params (NowColor :type EN_TraficLightState%20Enum :default "NewEnumerator0"))
  (switch Utilities|FlowControl|Switch|SwitchonEN_TraficLightState NowColor
    (:NewEnumerator0
      (bind _enumvalue (|ForEachEN_IntersectionDirection :!label _label)
        (:LoopBody
          (Utilities|IsValid (.Value (Utilities|Map|Find (Variables|Default|GetmTraficLights) _enumvalue))
            (:Is%20Valid
              (switch Utilities|FlowControl|Switch|SwitchonEN_TraficLightState NowColor
                (:NewEnumerator0
                  (if (Utilities|IsColorBlue (.Value (Utilities|Map|Find (Variables|Default|GetmTraficLights) _enumvalue)))
                    (Default|ChangeLightColor (.Value (Utilities|Map|Find (Variables|Default|GetmTraficLights) _enumvalue)) "NewEnumerator3")))
                (:NewEnumerator3
                  (if (Utilities|IsColorYerrow (.Value (Utilities|Map|Find (Variables|Default|GetmTraficLights) _enumvalue)))
                    (Default|ChangeLightColor (.Value (Utilities|Map|Find (Variables|Default|GetmTraficLights) _enumvalue)) "NewEnumerator7")))))))))
    (:NewEnumerator3
      (goto _label))
    (:NewEnumerator7
      (Private|SetBlueColorLight)
      (for _array_element (Variables|Default|GetmNowBlueLight)
        (Utilities|IsValid _array_element
          (:Is%20Valid
            (Default|ChangeLightColor _array_element "NewEnumerator0")))))))

(fn ClearBlueLight
  (Utilities|Array|Clear (Variables|Default|GetmNowBlueLight)))

(fn AddBlueLight
  (params (traficLight :type BP%20Trafic%20Light%20Object%20Reference) (traficLight2 :type BP%20Trafic%20Light%20Object%20Reference))
  (Utilities|FlowControl|Sequence
    (:then_0
      (Utilities|IsValid traficLight
        (:Is%20Valid
          (Utilities|Array|Add (Variables|Default|GetmNowBlueLight) traficLight))))
    (:then_1
      (Utilities|IsValid traficLight2
        (:Is%20Valid
          (Utilities|Array|Add (Variables|Default|GetmNowBlueLight) traficLight2))))))

(fn SetBlueColorLight
  (Utilities|FlowControl|Sequence
    (:then_0
      (bind _enumvalue (|ForEachEN_IntersectionDirection)
        (:LoopBody
          (if (== (Utilities|Array|FindItem (Variables|Default|GetmNowBlueLight) (.Value (Utilities|Map|Find (Variables|Default|GetmTraficLights) _enumvalue))) -1) ; 最近青ではなかった
            (Utilities|Array|Add (LocalVariables|GetinsArray) (.Value (Utilities|Map|Find (Variables|Default|GetmTraficLights) _enumvalue)))))))
    (:then_1
      (Private|ClearBlueLight)
      (Variables|Default|SetmNowBlueLight (LocalVariables|GetinsArray)))))