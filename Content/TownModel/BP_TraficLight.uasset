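; Traffic light for a town road junction that gates BP_CarBase traffic and links straight, right and left route splines.
; BeginPlay sets up child-actor road splines and registers only directions with a valid exit road on the shift splines.
; ChangeLightColor swaps lamp materials and enables the RedStop blocker on yellow or red.
; A looping frame-rate timer enables the RightCheck blocker while the light is blue and cars overlap Box.
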(event Custom|SetRightCheckCollision
  (bind _box (Variables|Default|GetBox))
  (CallFunction|SetCollisionEventUnBind)
  (Utilities|IsValid _box
    (:Is%20Valid
      (Collision|BindEventtoOnComponentBeginOverlap _box (delegate Custom|ObstacleBeginOverlap))
      (Collision|BindEventtoOnComponentEndOverlap _box (delegate Custom|ObstacleEndOverlap)))))

(event Custom|ObstacleBeginOverlap
  (params (OverlappedComponent :type Primitive%20Component%20Object%20Reference) (OtherActor :type Actor%20Object%20Reference) (OtherComp :type Primitive%20Component%20Object%20Reference) (OtherBodyIndex :type Integer) (bFromSweep :type Boolean) (SweepResult :type Hit%20Result%20Structure%20%28by%20ref%29))
  (Utilities|Casting|CastToBP_CarBase OtherActor)
  (if (not (Variables|Default|GetmRightCheck))
    (Variables|Default|SetmRightCheck true)))

(event Custom|ObstacleEndOverlap
  (params (OverlappedComponent :type Primitive%20Component%20Object%20Reference) (OtherActor :type Actor%20Object%20Reference) (OtherComp :type Primitive%20Component%20Object%20Reference) (OtherBodyIndex :type Integer))
  (if (and (Variables|Default|GetmRightCheck) (<= (Utilities|Array|Length (Collision|GetOverlappingActors (Variables|Default|GetBox) "/Game/TownModel/BP_CarBase.BP_CarBase_C" :!class /Script/Engine.PrimitiveComponent)) 0))
    (Variables|Default|SetmRightCheck false)))

(event Custom|SetCollisionEventUnBind
  (bind _box (Variables|Default|GetBox))
  (Utilities|IsValid _box
    (:Is%20Valid
      (Collision|UnbindEventfromOnComponentBeginOverlap _box (EventDispatchers|CreateEvent :!event Custom|ObstacleBeginOverlap))
      (Collision|UnbindEventfromOnComponentEndOverlap _box (EventDispatchers|CreateEvent :!event Custom|ObstacleEndOverlap)))))

(event Custom|TIck
  (bind _rightcheck (Variables|Default|GetRightCheck))
  (if (and (Utilities|Enum|Equal(Enum) (Variables|Default|GetmColorState) "NewEnumerator0") (Variables|Default|GetmRightCheck))
    (Collision|SetCollisionEnabled _rightcheck "QueryAndPhysics")
    (Development|SetHiddeninGame _rightcheck false false)
    (else
      (Collision|SetCollisionEnabled _rightcheck "NoCollision")
      (Development|SetHiddeninGame _rightcheck true false))))

(event EventBeginPlay
  (Private|SetDirection)
  (CallFunction|SetRightCheckCollision)
  (Utilities|Time|SetTimerbyEvent (delegate Custom|TIck) 0.016667 true))

(event EventTick
  (params (DeltaSeconds :type Float%20%28single-precision%29)))

(fn ConstructionScript)

(fn SetDirection
  (Utilities|FlowControl|Sequence
    (:then_0
      (Default|SetSpline (Utilities|GetRoadSpline (Variables|Default|GetStraightRoadSpline)) (Variables|Default|GetStraightSpline))
      (Default|SetSpline (Utilities|GetRoadSpline (Variables|Default|GetRightRoadSpline)) (Variables|Default|GetRightSpline))
      (Default|SetSpline (Utilities|GetRoadSpline (Variables|Default|GetLeftRoadSpline)) (Variables|Default|GetLeftSpline)))
    (:then_1
      (Private|SetDirectionSpline (Variables|Default|GetStraightShiftSpline) (Variables|Default|GetStraightRoadSpline) (Variables|Default|GetmShiftStraight))
      (Private|SetDirectionSpline (Variables|Default|GetRightShiftSpline) (Variables|Default|GetRightRoadSpline) (Variables|Default|GetmShiftRight))
      (Private|SetDirectionSpline (Variables|Default|GetLeftShiftSpline) (Variables|Default|GetLeftRoadSpline) (Variables|Default|GetmShiftLeft)))))

(fn AddParentSplines
  (params (ShiftSpline :type BP%20Shift%20Spline%20Object%20Reference) (RoadSpline :type BP%20Road%20Spline%20Object%20Reference%20%28by%20ref%29))
  (Utilities|IsValid RoadSpline
    (:Is%20Valid
      (Utilities|Array|Add (Variables|/Game/Spline/BP_ShiftSpline.BP_ShiftSpline_C|GetmParentSplines ShiftSpline) RoadSpline)
      (return true))
    (:Is%20Not%20Valid
      (return false))))

(fn SetDirectionSpline
  (params (ShiftSpline :type Child%20Actor%20Component%20Object%20Reference) (TraficLightRoadSpline :type Child%20Actor%20Component%20Object%20Reference) (AfterRoadSpline :type BP%20Road%20Spline%20Object%20Reference%20%28by%20ref%29))
  (bind _success (Private|AddParentSplines (Utilities|GetShiftSpline ShiftSpline) AfterRoadSpline))
  (if _success
    (Private|AddParentSplines (Utilities|GetDirectionBox) (Utilities|GetRoadSpline TraficLightRoadSpline))))

(fn ChangeLightColor
  (params (Color :type EN_TraficLightState%20Enum :default "NewEnumerator0"))
  (bind _redstop (Variables|Default|GetRedStop))
  (bind _redstop_2 (Variables|Default|GetRedStop))
  (Utilities|FlowControl|Sequence
    (:then_0
      (Variables|Default|SetmColorState Color))
    (:then_1
      (switch Utilities|FlowControl|Switch|SwitchonEN_TraficLightState Color
        (:NewEnumerator0
          (Rendering|Material|SetMaterial (Variables|Default|GetColorRed1) 0 "/Game/TownModel/TraficLight/Trafic_Black.Trafic_Black")
          (Rendering|Material|SetMaterial (Variables|Default|GetColorRed2) 0 "/Game/TownModel/TraficLight/Trafic_Black.Trafic_Black")
          (Rendering|Material|SetMaterial (Variables|Default|GetColorYerrow1) 0 "/Game/TownModel/TraficLight/Trafic_Black.Trafic_Black")
          (Rendering|Material|SetMaterial (Variables|Default|GetColorYerrow2) 0 "/Game/TownModel/TraficLight/Trafic_Black.Trafic_Black")
          (Rendering|Material|SetMaterial (Variables|Default|GetColorBlue1) 0 "/Game/TownModel/TraficLight/Trafic_Blue.Trafic_Blue")
          (Rendering|Material|SetMaterial (Variables|Default|GetColorBlue2) 0 "/Game/TownModel/TraficLight/Trafic_Blue.Trafic_Blue")
          (Collision|SetCollisionEnabled _redstop_2 "NoCollision")
          (Development|SetHiddeninGame _redstop_2 true false))
        (:NewEnumerator3
          (Rendering|Material|SetMaterial (Variables|Default|GetColorRed1) 0 "/Game/TownModel/TraficLight/Trafic_Black.Trafic_Black")
          (Rendering|Material|SetMaterial (Variables|Default|GetColorRed2) 0 "/Game/TownModel/TraficLight/Trafic_Black.Trafic_Black")
          (Rendering|Material|SetMaterial (Variables|Default|GetColorYerrow1) 0 "/Game/TownModel/TraficLight/Trafic_Yerrow.Trafic_Yerrow")
          (Rendering|Material|SetMaterial (Variables|Default|GetColorYerrow2) 0 "/Game/TownModel/TraficLight/Trafic_Yerrow.Trafic_Yerrow")
          (Rendering|Material|SetMaterial (Variables|Default|GetColorBlue1) 0 "/Game/TownModel/TraficLight/Trafic_Black.Trafic_Black")
          (Rendering|Material|SetMaterial (Variables|Default|GetColorBlue2) 0 "/Game/TownModel/TraficLight/Trafic_Black.Trafic_Black")
          (Collision|SetCollisionEnabled _redstop "QueryAndPhysics" :!label _label)
          (Development|SetHiddeninGame _redstop false false))
        (:NewEnumerator7
          (Rendering|Material|SetMaterial (Variables|Default|GetColorRed1) 0 "/Game/TownModel/TraficLight/Trafic_Red.Trafic_Red")
          (Rendering|Material|SetMaterial (Variables|Default|GetColorRed2) 0 "/Game/TownModel/TraficLight/Trafic_Red.Trafic_Red")
          (Rendering|Material|SetMaterial (Variables|Default|GetColorYerrow1) 0 "/Game/TownModel/TraficLight/Trafic_Black.Trafic_Black")
          (Rendering|Material|SetMaterial (Variables|Default|GetColorYerrow2) 0 "/Game/TownModel/TraficLight/Trafic_Black.Trafic_Black")
          (Rendering|Material|SetMaterial (Variables|Default|GetColorBlue1) 0 "/Game/TownModel/TraficLight/Trafic_Black.Trafic_Black")
          (Rendering|Material|SetMaterial (Variables|Default|GetColorBlue2) 0 "/Game/TownModel/TraficLight/Trafic_Black.Trafic_Black")
          (goto _label))))))