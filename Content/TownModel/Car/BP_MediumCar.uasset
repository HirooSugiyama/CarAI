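; BP_MediumCar is a medium-car child Blueprint in the town car models, specializing a parent car class.
; It overrides SetCarModel to call the parent, then assign the car mesh a random entry from the medium-car map, looked up by a 1-based integer key.
; GetAccelSpeed returns a random speed within the range around the base speed.
; The event graph holds only disabled placeholder events.
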(event EventBeginPlay
  (|CallParentFunction) ; このノードは無効になっているため呼び出せません。\n機能をビルドするにはピンをドラッグしてください。
)

(event Collision|EventActorBeginOverlap
  (params (OtherActor :type Actor%20Object%20Reference)))

(event EventTick
  (params (DeltaSeconds :type Float%20%28single-precision%29)))

(fn ConstructionScript
  (|CallParentFunction))

(fn SetCarModel
  (|CallParentFunction)
  (Components|StaticMesh|SetStaticMesh (Variables|Default|GetCarModel) (.Value (Utilities|Map|Find (LocalVariables|GetMEDIUM_CAR_MAP) (+ (Math|Random|RandomInteger (Utilities|Map|Length (LocalVariables|GetMEDIUM_CAR_MAP))) 1)))))

(fn GetAccelSpeed
  (return (Math|Random|RandomFloatinRange (- (LocalVariables|GetBASE_SPEED) (LocalVariables|GetSPEED_RANGE)) (+ (LocalVariables|GetBASE_SPEED) (LocalVariables|GetSPEED_RANGE)))))