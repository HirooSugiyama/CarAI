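; Base Blueprint for a town-model car that moves along a spline through its SplineMoveComponent.
; Initialize sets the model, hands the front box to the component for collision detection and binds MoveDelay, which clears the collision stop after a GetAccelSpeed-length wait.
; SetMaxSpeed, Accelerator and Stop drive the component's speed directly.
; SetCarModel and GetAccelSpeed are stubs here, and the construction script's mesh assignment is disconnected.
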(event Custom|MoveDelay
  (bind _speed (Protected|GetAccelSpeed))
  (Utilities|FlowControl|Delay _speed)
  (Variables|/Game/TownModel/SplineMoveComponent.SplineMoveComponent_C|SetCollisionStop (Variables|Default|GetSplineMoveComponent) false))

(event Custom|Initialize
  (bind _splinemovecomponent (Variables|Default|GetSplineMoveComponent))
  (Protected|SetCarModel)
  (Default|SetCollisionEvent _splinemovecomponent (Variables|Default|GetFrontBox))
  (EventDispatchers|BindEventtoMoveDelay _splinemovecomponent (delegate Custom|MoveDelay)))

(event EventBeginPlay)

(fn ConstructionScript)

(fn SetMaxSpeed
  (params (mMaxSpeed :type Float%20%28single-precision%29))
  (bind _output_get (Variables|Default|SetmMaxSpeed mMaxSpeed))
  (Variables|/Game/TownModel/SplineMoveComponent.SplineMoveComponent_C|SetSpeed (Variables|Default|GetSplineMoveComponent) _output_get) ; DEBUG
)

(fn Accelerator
  (Variables|/Game/TownModel/SplineMoveComponent.SplineMoveComponent_C|SetSpeed (Variables|Default|GetSplineMoveComponent) (Variables|Default|GetmMaxSpeed)) ; DEBUG
)

(fn Stop
  (Variables|/Game/TownModel/SplineMoveComponent.SplineMoveComponent_C|SetSpeed (Variables|Default|GetSplineMoveComponent) 0.0))

(fn SetCarModel)

(fn GetAccelSpeed
  (return 0.0))