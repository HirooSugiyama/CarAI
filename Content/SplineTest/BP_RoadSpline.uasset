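; BP_RoadSpline is a road path Blueprint that wraps a spline for distance-based queries.
; GetCurrentLocationAndRotation returns world location and rotation at a given distance, using modulo to wrap around the spline length when looping.
; Its Direction output is fed by the same location lookup as Location, not a direction.
; IsArrived checks whether a distance has reached the spline's end, and SetSpline assigns the spline; event and construction graphs are empty.
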(event EventBeginPlay)

(event Collision|EventActorBeginOverlap
  (params (OtherActor :type Actor%20Object%20Reference)))

(event EventTick
  (params (DeltaSeconds :type Float%20%28single-precision%29)))

(fn ConstructionScript)

(fn GetCurrentLocationandRotation
  (params (Length :type Float%20%28single-precision%29) (loop :type Boolean))
  (bind _spline (Variables|Default|GetSpline))
  (if loop
    (LocalVariables|SetlocalLength (Math|Float|%(Float) Length (Spline|GetSplineLength (Variables|Default|GetSpline))))
    (else
      (LocalVariables|SetlocalLength Length)))
  (return (Spline|GetLocationatDistanceAlongSpline _spline (LocalVariables|GetlocalLength) "World") (Spline|GetLocationatDistanceAlongSpline _spline (LocalVariables|GetlocalLength) "World") (Spline|GetRotationatDistanceAlongSpline _spline (LocalVariables|GetlocalLength) "World")))

(fn IsArrived
  (params (Length :type Float%20%28single-precision%29))
  (return (>= Length (Spline|GetSplineLength (Variables|Default|GetSpline)))))

(fn SetSpline
  (params (Spline :type Spline%20Component%20Object%20Reference))
  (Variables|Default|SetSpline Spline))