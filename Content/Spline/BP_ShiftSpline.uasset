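; BP_ShiftSpline is a trigger actor that switches an overlapping BP_CarBase onto a random road spline from MParentSplines.
; On overlap, it hands the chosen spline and the car's matching distance along it to the car's SplineMoveComponent.
; That distance is approximated by interpolating between neighbouring spline point distances using straight-line length ratios.
; A separate DEBUG function spawns a cube-mesh BP_House at a given location.
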(event Collision|EventActorBeginOverlap
  (params (OtherActor :type Actor%20Object%20Reference))
  (if (Utilities|Array|IsValidIndex (Variables|Default|GetmParentSplines))
    (bind _asbp_car_base (Utilities|Casting|CastToBP_CarBase OtherActor))
    (bind _output (CallFunction|RandomSpline))
    (Default|SetRoadSpline (Variables|/Game/TownModel/BP_CarBase.BP_CarBase_C|GetSplineMoveComponent _asbp_car_base) _output)
    (bind _returnvalue (CallFunction|Calculate%AlongSplinefromClosestWorldLocation (Transformation|GetActorLocation _asbp_car_base) (Variables|/Game/Spline/BP_RoadSpline.BP_RoadSpline_C|GetSpline _output)))
    (Default|SetMoveDistance (Variables|/Game/TownModel/BP_CarBase.BP_CarBase_C|GetSplineMoveComponent _asbp_car_base) _returnvalue)))

(fn ConstructionScript)

(fn RandomSpline
  (bind _mparentsplines (Variables|Default|GetmParentSplines))
  (return (Utilities|Array|Get(acopy) _mparentsplines (Math|Random|RandomInteger (Utilities|Array|Length _mparentsplines)))))

(fn Calculate%AlongSplinefromClosestWorldLocation
  (params (The%20Location :type Vector) (InputPin :type Spline%20Component%20Object%20Reference))
  (LocalVariables|SetTheLocation The%20Location)
  (LocalVariables|SetThe%20Spline InputPin)
  (bind _output_get (LocalVariables|SetKey%20ID (Math|Float|Truncate (Class|SplineComponent|FindInputKeyClosesttoWorldLocation (LocalVariables|GetThe%20Spline) (LocalVariables|GetTheLocation)))))
  (return (Math|Float|Lerp (Spline|GetDistanceAlongSplineatSplinePoint (LocalVariables|GetThe%20Spline) _output_get) (Spline|GetDistanceAlongSplineatSplinePoint (LocalVariables|GetThe%20Spline) (+ _output_get 1)) (/ (Math|Vector|VectorLength (- (Spline|FindLocationClosesttoWorldLocation (LocalVariables|GetThe%20Spline) (LocalVariables|GetTheLocation) "World") (Spline|GetLocationatSplinePoint (LocalVariables|GetThe%20Spline) (LocalVariables|GetKey%20ID) "World"))) (Math|Vector|VectorLength (- (Spline|GetLocationatSplinePoint (LocalVariables|GetThe%20Spline) (+ (LocalVariables|GetKey%20ID) 1) "World") (Spline|GetLocationatSplinePoint (LocalVariables|GetThe%20Spline) (LocalVariables|GetKey%20ID) "World")))))))

(fn DEBUG
  (params (NewParam :type Vector))
  (bind _returnvalue (Game|SpawnActorfromClass "/Game/TownModel/BP_House.BP_House_C" (Math|Transform|MakeTransform NewParam "0, 0, 0" "1,1,1") "Undefined" 0 0))
  (Variables|/Game/TownModel/BP_House.BP_House_C|SethouseSrtaticMeshModel _returnvalue "/Game/TownModel/TraficLight/1M_Cube.1M_Cube"))